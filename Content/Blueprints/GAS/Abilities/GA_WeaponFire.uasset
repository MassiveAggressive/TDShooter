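; Gameplay ability that fires the TDSCharacter's weapon, supporting single-shot and automatic fire.
; Activation commits and fires once, then either ends or, for automatic weapons, repeats on an attribute-timed delay, recommitting each shot until input release or commit failure.
; Each shot spawns an attribute-driven number of projectiles with attribute-based damage and random yaw-only cone spread, reporting an AI noise event per projectile.
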(event `self.K2_ActivateAbility`
  (bind _astdscharacter (cast `TDSCharacter` (`self.GetAvatarActorFromActorInfo`)))
  (set `self.IsAutoFire` (`TDSWeapon.IsAutoFire` (`TDSCharacter.Weapon` _astdscharacter)))
  (`self.K2_CommitAbility`)
  (`self.Fire`)
  (if (`self.IsAutoFire`)
    (`AbilityTask_WaitInputRelease.WaitInputRelease` false
      (:`then`
        (`GameplayTask_WaitDelay.TaskWaitDelay` null (/ 1.0 (`.ReturnValue` (`AbilitySystemComponent.GetGameplayAttributeValue` (`self.GetAbilitySystemComponentFromActorInfo`) (struct :`AttributeName` "FiringRate" :`Attribute` "/Script/TDShooter.TDSWeaponSet:FiringRate" :`AttributeOwner` "/Script/CoreUObject.Class'/Script/TDShooter.TDSWeaponSet'")))) :!label _label
          (:`OnFinish`
            (bind _returnvalue (`self.K2_CommitAbility`))
            (if _returnvalue
              (`self.Fire`)
              (goto _label)
              (else
                (`self.K2_EndAbility`))))))
      (:`OnRelease`
        (`self.K2_EndAbility` :!label _label_2)))
    (else
      (goto _label_2))))

(fn `Fire`
  (locals (RotationRef :type "Rotator Structure" :default (struct)))
  (bind _returnvalue (`self.GetAvatarActorFromActorInfo`))
  (bind (_returnvalue_roll _returnvalue_pitch _returnvalue_yaw) (`KismetMathLibrary.BreakRotator` (`KismetMathLibrary.Conv_VectorToRotator` (`KismetMathLibrary.RandomUnitVectorInConeInDegrees` (`Actor.GetActorForwardVector` (`self.GetAvatarActorFromActorInfo`)) (`.ReturnValue` (`AbilitySystemComponent.GetGameplayAttributeValue` (`self.GetAbilitySystemComponentFromActorInfo`) (struct :`AttributeName` "ShotSpread" :`Attribute` "/Script/TDShooter.TDSWeaponSet:ShotSpread" :`AttributeOwner` "/Script/CoreUObject.Class'/Script/TDShooter.TDSWeaponSet'")))))))
  (for _ (range (+ (`KismetMathLibrary.FTrunc` (- (`.ReturnValue` (`AbilitySystemComponent.GetGameplayAttributeValue` (`self.GetAbilitySystemComponentFromActorInfo`) (struct :`AttributeName` "ShotCount" :`Attribute` "/Script/TDShooter.TDSWeaponSet:ShotCount" :`AttributeOwner` "/Script/CoreUObject.Class'/Script/TDShooter.TDSWeaponSet'"))) 1.0)) 1))
    (set `local.RotationRef` (`KismetMathLibrary.MakeRotator` 0.0 0.0 _returnvalue_yaw))
    (`|SpawnActorFromClass` (`self.ProjectileClass`) (`KismetMathLibrary.MakeTransform` (`Actor.K2_GetActorLocation` _returnvalue) (`local.RotationRef`)) "AlwaysSpawn" "MultiplyWithRoot" _returnvalue (`.ReturnValue` (`AbilitySystemComponent.GetGameplayAttributeValue` (`self.GetAbilitySystemComponentFromActorInfo`) (struct :`AttributeName` "Damage" :`Attribute` "/Script/TDShooter.TDSWeaponSet:Damage" :`AttributeOwner` "/Script/CoreUObject.Class'/Script/TDShooter.TDSWeaponSet'"))) null)
    (`AISense_Hearing.ReportNoiseEvent` (`Actor.K2_GetActorLocation` (`self.GetAvatarActorFromActorInfo`)) 1.0 (`self.GetAvatarActorFromActorInfo`))))