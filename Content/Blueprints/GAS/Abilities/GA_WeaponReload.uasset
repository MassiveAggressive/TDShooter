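; GA_WeaponReload is a gameplay ability that reloads a weapon by moving carried ammo into the loaded count, then ends immediately.
; It reads loaded, max loaded and carried ammo from the avatar's Ability System Component and transfers the smaller of carried ammo and free space.
; The new totals, rather than deltas, go into a GE_AmmoUpdate spec through SetByCaller tags, which is applied to the avatar.
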(event `self.K2_ActivateAbility`
  (`self.K2_CommitAbility`)
  (`self.Reload`)
  (`self.K2_EndAbility`))

(fn `Reload`
  (locals (AvatarASC :type "AbilitySystemComponent Object Reference") (LoadedAmmoRef :type "Float (single-precision)" :default 0.0) (MaxLoadedAmmoRef :type "Float (single-precision)" :default 0.0) (CarriedAmmoRef :type "Float (single-precision)" :default 0.0) (LoadingAmmo :type "Float (double-precision)"))
  (set `local.AvatarASC` (`AbilitySystemBlueprintLibrary.GetAbilitySystemComponent` (`self.GetAvatarActorFromActorInfo`)))
  (`|ExecutionSequence`
    (:`then_0`
      (set `local.LoadedAmmoRef` (`.ReturnValue` (`AbilitySystemComponent.GetGameplayAttributeValue` (`local.AvatarASC`) (struct :`AttributeName` "LoadedAmmo" :`Attribute` "/Script/TDShooter.TDSWeaponSet:LoadedAmmo" :`AttributeOwner` "/Script/CoreUObject.Class'/Script/TDShooter.TDSWeaponSet'"))))
      (set `local.MaxLoadedAmmoRef` (`.ReturnValue` (`AbilitySystemComponent.GetGameplayAttributeValue` (`local.AvatarASC`) (struct :`AttributeName` "MaxLoadedAmmo" :`Attribute` "/Script/TDShooter.TDSWeaponSet:MaxLoadedAmmo" :`AttributeOwner` "/Script/CoreUObject.Class'/Script/TDShooter.TDSWeaponSet'"))))
      (set `local.CarriedAmmoRef` (`.ReturnValue` (`AbilitySystemComponent.GetGameplayAttributeValue` (`local.AvatarASC`) (struct :`AttributeName` "CarriedAmmo" :`Attribute` "/Script/TDShooter.TDSWeaponSet:CarriedAmmo" :`AttributeOwner` "/Script/CoreUObject.Class'/Script/TDShooter.TDSWeaponSet'")))))
    (:`then_1`
      (set `local.LoadingAmmo` (`KismetMathLibrary.FMin` (`local.CarriedAmmoRef`) (- (`local.MaxLoadedAmmoRef`) (`local.LoadedAmmoRef`))))
      (set `local.LoadedAmmoRef` (+ (`local.LoadedAmmoRef`) (`local.LoadingAmmo`)))
      (set `local.CarriedAmmoRef` (- (`local.CarriedAmmoRef`) (`local.LoadingAmmo`))))
    (:`then_2`
      (bind _returnvalue (`AbilitySystemBlueprintLibrary.AssignTagSetByCallerMagnitude` (`AbilitySystemComponent.MakeOutgoingSpec` :`self` (`local.AvatarASC`) :`GameplayEffectClass` "/Game/Blueprints/GAS/Effects/GE_AmmoUpdate.GE_AmmoUpdate_C") (struct :`TagName` "Ammo.Loaded.SetByCaller") (`local.LoadedAmmoRef`)))
      (bind _returnvalue_2 (`AbilitySystemBlueprintLibrary.AssignTagSetByCallerMagnitude` _returnvalue (struct :`TagName` "Ammo.Carried.SetByCaller") (`local.CarriedAmmoRef`)))
      (`AbilitySystemComponent.BP_ApplyGameplayEffectSpecToSelf` (`local.AvatarASC`) _returnvalue_2))))