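; Base weapon pickup that a TDSCharacter equips when it overlaps the sphere.
; On equip it grants fire, alt and reload abilities to the owner's Ability System Component with input IDs.
; It then applies set-by-caller gameplay effects to initialize weapon stats and update ammo, sending zero loaded and a sum of two attributes as carried.
; Unequip clears the fire and alt abilities but leaves reload granted.
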(event `self.OnEquip`
  (bind _ownerasc (`self.OwnerASC`))
  (`KismetSystemLibrary.PrintString` (`KismetStringLibrary.Concat_StrStr` (`KismetSystemLibrary.GetDisplayName` self) " equipped"))
  (set `self.OwnerASC` (`AbilitySystemBlueprintLibrary.GetAbilitySystemComponent` (`self.GetOwner`)))
  (`|ExecutionSequence`
    (:`then_0`
      (bind _returnvalue (`AbilitySystemComponent.K2_GiveAbility` (`self.OwnerASC`) (`self.WeaponFireAbilityClass`) 0 (`KismetMathLibrary.Conv_ByteToInt` (`self.WeaponFireAbilityInputID`))))
      (set `self.WeaponFireAbilityHandle` _returnvalue))
    (:`then_1`
      (bind _returnvalue_2 (`AbilitySystemComponent.K2_GiveAbility` (`self.OwnerASC`) (`self.WeaponAltAbilityClass`) 0 (`KismetMathLibrary.Conv_ByteToInt` (`self.WeaponAltAbilityInputID`))))
      (set `self.WeaponAltAbilityHandle` _returnvalue_2))
    (:`then_2`
      (bind _returnvalue_3 (`AbilitySystemComponent.K2_GiveAbility` (`self.OwnerASC`) (`self.WeaponReloadAbilityClass`) 0 (`KismetMathLibrary.Conv_ByteToInt` (`self.WeaponReloadAbilityInputID`))))
      (set `self.WeaponReloadAbilityHandle` _returnvalue_3))
    (:`then_3`
      (bind _returnvalue_4 (`AbilitySystemBlueprintLibrary.AssignTagSetByCallerMagnitude` (`AbilitySystemComponent.MakeOutgoingSpec` :`self` (`self.OwnerASC`) :`GameplayEffectClass` "/Game/Blueprints/GAS/Effects/GE_InitWeaponSet.GE_InitWeaponSet_C") (struct :`TagName` "WeaponSet.Init.Damage") (`self.Damage`)))
      (bind _returnvalue_5 (`AbilitySystemBlueprintLibrary.AssignTagSetByCallerMagnitude` _returnvalue_4 (struct :`TagName` "WeaponSet.Init.FiringRate") (`self.FiringRate`)))
      (bind _returnvalue_6 (`AbilitySystemBlueprintLibrary.AssignTagSetByCallerMagnitude` _returnvalue_5 (struct :`TagName` "WeaponSet.Init.MaxLoadedAmmo") (`self.MaxLoadedAmmo`)))
      (bind _returnvalue_7 (`AbilitySystemBlueprintLibrary.AssignTagSetByCallerMagnitude` _returnvalue_6 (struct :`TagName` "WeaponSet.Init.ShotCount") (`self.ShotCount`)))
      (bind _returnvalue_8 (`AbilitySystemBlueprintLibrary.AssignTagSetByCallerMagnitude` _returnvalue_7 (struct :`TagName` "WeaponSet.Init.ShotSpread") (`self.ShotSpread`)))
      (`AbilitySystemComponent.BP_ApplyGameplayEffectSpecToSelf` (`self.OwnerASC`) _returnvalue_8))
    (:`then_4`
      (bind _returnvalue_9 (`AbilitySystemBlueprintLibrary.AssignTagSetByCallerMagnitude` (`AbilitySystemComponent.MakeOutgoingSpec` :`self` (`self.OwnerASC`) :`GameplayEffectClass` "/Game/Blueprints/GAS/Effects/GE_AmmoUpdate.GE_AmmoUpdate_C") (struct :`TagName` "Ammo.Loaded.SetByCaller")))
      (bind _returnvalue_10 (`AbilitySystemBlueprintLibrary.AssignTagSetByCallerMagnitude` _returnvalue_9 (struct :`TagName` "Ammo.Carried.SetByCaller") (+ (`.ReturnValue` (`AbilitySystemComponent.GetGameplayAttributeValue` _ownerasc (struct :`AttributeName` "CarriedAmmo" :`Attribute` "/Script/TDShooter.TDSWeaponSet:CarriedAmmo" :`AttributeOwner` "/Script/CoreUObject.Class'/Script/TDShooter.TDSWeaponSet'"))) (`.ReturnValue` (`AbilitySystemComponent.GetGameplayAttributeValue` _ownerasc (struct :`AttributeName` "LoadedAmmo" :`Attribute` "/Script/TDShooter.TDSWeaponSet:LoadedAmmo" :`AttributeOwner` "/Script/CoreUObject.Class'/Script/TDShooter.TDSWeaponSet'"))))))
      (`AbilitySystemComponent.BP_ApplyGameplayEffectSpecToSelf` (`self.OwnerASC`) _returnvalue_10))))

(event `self.OnUnEquip`
  (`KismetSystemLibrary.PrintString` (`KismetStringLibrary.Concat_StrStr` (`KismetSystemLibrary.GetDisplayName` self) " unequipped"))
  (`AbilitySystemComponent.ClearAbility` (`self.OwnerASC`) (`self.WeaponFireAbilityHandle`))
  (`AbilitySystemComponent.ClearAbility` (`self.OwnerASC`) (`self.WeaponAltAbilityHandle`)))

(event `self.Sphere.OnComponentBeginOverlap`
  (params (OverlappedComponent :type "PrimitiveComponent Object Reference") (OtherActor :type "Actor Object Reference") (OtherComp :type "PrimitiveComponent Object Reference") (OtherBodyIndex :type Integer) (bFromSweep :type Boolean) (SweepResult :type "HitResult Structure (by ref)"))
  (bind _astdscharacter (cast `TDSCharacter` OtherActor))
  (`TDSCharacter.EquipWeapon` _astdscharacter self))

(fn `UserConstructionScript`)