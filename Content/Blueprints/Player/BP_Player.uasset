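; BP_Player is the player pawn, which moves on world X/Y through Enhanced Input and turns to face a hit location.
; On BeginPlay it adds the input mapping, creates the HUD and spawns a BP_Ground that snaps to its position while keeping world rotation.
; Each Tick sets yaw toward GetHitLocation, independent of movement direction.
; Health and shield change events are relayed through their Call functions.
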(event `self.ReceiveBeginPlay`
  (`EnhancedInputSubsystemInterface.AddMappingContext` (pcsubsystem `EnhancedInputLocalPlayerSubsystem` (`GameplayStatics.GetPlayerController` 0)) "/Game/Inputs/IMC_General.IMC_General" 0 (struct))
  (bind _returnvalue (`|SpawnActorFromClass` "/Game/Blueprints/Player/BP_Ground.BP_Ground_C" (`KismetMathLibrary.MakeTransform` (`self.K2_GetActorLocation`)) "AlwaysSpawn" "MultiplyWithRoot" null null))
  (`self.K2_AttachToActor` _returnvalue self "None" "SnapToTarget" "KeepWorld" "KeepWorld" true)
  (bind _returnvalue_2 (`|CreateWidget` "/Game/Blueprints/Player/W_HUD.W_HUD_C" null self))
  (bind _output_get (set `self.HUD` _returnvalue_2))
  (`UserWidget.AddToViewport` _output_get 0))

(event `self.ReceiveTick`
  (params (DeltaSeconds :type "Float (single-precision)"))
  (bind (_location_x _location_y) (`KismetMathLibrary.BreakVector` (`/Game/Blueprints/Functions/GeneralFunctions.GetHitLocation`)))
  (bind (_returnvalue_x _returnvalue_y) (`KismetMathLibrary.BreakVector` (`self.K2_GetActorLocation`)))
  (bind (_returnvalue_roll _returnvalue_pitch _returnvalue_yaw) (`KismetMathLibrary.BreakRotator` (`KismetMathLibrary.FindLookAtRotation` (`KismetMathLibrary.MakeVector` _returnvalue_x _returnvalue_y) (`KismetMathLibrary.MakeVector` _location_x _location_y))))
  (`self.K2_SetActorRotation` (`KismetMathLibrary.MakeRotator` 0.0 0.0 _returnvalue_yaw)))

(event `EnhancedInput|/Game/Inputs/IA_Move`
  (params (ActionValue :type "Vector2D Structure") (ElapsedSeconds :type "Float (double-precision)") (TriggeredSeconds :type "Float (double-precision)") (InputAction :type "InputAction Object Reference" :default "/Game/Inputs/IA_Move.IA_Move"))
  (:`Triggered`
    (`self.AddMovementInput` (`KismetMathLibrary.MakeVector` ActionValue_X ActionValue_Y) :!label _label))
  (:`Started`
    (goto _label))
  (:`Ongoing`
    (goto _label))
  (:`Canceled`
    (goto _label))
  (:`Completed`
    (goto _label)))

(event `self.OnHealthChanged`
  (params (OldValue :type "Float (single-precision)") (NewValue :type "Float (single-precision)"))
  (`self.OnHealthChangedEvent`))

(event `self.OnShieldChanged`
  (params (OldValue :type "Float (single-precision)") (NewValue :type "Float (single-precision)"))
  (`self.OnShieldChangedEvent`))

(fn `UserConstructionScript`)