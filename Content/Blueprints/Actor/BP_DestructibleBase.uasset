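; Base destructible actor that uses the Gameplay Ability System for health, shaking when hurt and destroying itself at zero.
; On BeginPlay it applies GE_InitHealthSet to itself, passing StartingHealth as a SetByCaller max-health magnitude.
; Health changes that leave it above zero trigger a brief shake: a small local rotation, reversed after a short delay.
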(event `self.ReceiveBeginPlay`
  (bind _returnvalue (`AbilitySystemBlueprintLibrary.AssignTagSetByCallerMagnitude` (`AbilitySystemComponent.MakeOutgoingSpec` :`self` (`self.AbilitySystemComponent`) :`GameplayEffectClass` "/Game/Blueprints/GAS/Effects/GE_InitHealthSet.GE_InitHealthSet_C") (struct :`TagName` "HealthSet.Init.MaxHealth") (`self.StartingHealth`)))
  (`AbilitySystemComponent.BP_ApplyGameplayEffectSpecToSelf` (`self.AbilitySystemComponent`) _returnvalue))

(event `self.OnHealthChanged`
  (params (OldValue :type "Float (single-precision)") (NewValue :type "Float (single-precision)"))
  (if (> NewValue 0.0)
    (`self.Shake`)
    (else
      (`self.K2_DestroyActor`))))

(event `Shake`
  (`self.K2_AddActorLocalRotation` (struct :`Yaw` 5.0))
  (`KismetSystemLibrary.Delay` 0.1)
  (`self.K2_AddActorLocalRotation` (struct :`Yaw` -5.0)))

(fn `UserConstructionScript`)