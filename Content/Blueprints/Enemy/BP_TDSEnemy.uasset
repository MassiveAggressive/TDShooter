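; Enemy character Blueprint driven by the Gameplay Ability System and AI, destroyed when its health runs out.
; BeginPlay initializes max health and shield through a SetByCaller init effect and copies AttackRange to the Blackboard.
; Damage taken is reported as an AI damage sense event, located at the damage causer's position.
; Attack activates the first default ability without using its target argument.
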(event `self.ReceiveBeginPlay`
  (bind _returnvalue (`AbilitySystemBlueprintLibrary.AssignTagSetByCallerMagnitude` (`AbilitySystemComponent.MakeOutgoingSpec` :`self` (`self.AbilitySystemComponent`) :`GameplayEffectClass` "/Game/Blueprints/GAS/Effects/GE_InitHealthSet.GE_InitHealthSet_C") (struct :`TagName` "HealthSet.Init.MaxHealth") 50.0))
  (bind _returnvalue_2 (`AbilitySystemBlueprintLibrary.AssignTagSetByCallerMagnitude` _returnvalue (struct :`TagName` "HealthSet.Init.MaxShield") 20.0))
  (`AbilitySystemComponent.BP_ApplyGameplayEffectSpecToSelf` (`self.AbilitySystemComponent`) _returnvalue_2)
  (`BlackboardComponent.SetValueAsFloat` (`AIBlueprintHelperLibrary.GetBlackboard` null) "AttackRange" (`self.AttackRange`)))

(event `self.OnHealthChanged`
  (params (OldValue :type "Float (single-precision)") (NewValue :type "Float (single-precision)"))
  (if (<= NewValue 0.0)
    (`self.K2_DestroyActor`)))

(event `self.OnDamageTaken`
  (params (DamageInstigator :type "Actor Object Reference") (DamageCauser :type "Actor Object Reference") (GameplayTagContainer :type "GameplayTagContainer Structure (by ref)") (Damage :type "Float (single-precision)"))
  (`AISense_Damage.ReportDamageEvent` self DamageInstigator Damage (`self.K2_GetActorLocation` DamageCauser)))

(fn `Attack`
  (params (TargetActor :type "Actor Object Reference"))
  (`AbilitySystemComponent.TryActivateAbilityByClass` (`self.AbilitySystemComponent`) (`|GetArrayItem` (`self.DefaultAbilities`)) true))

(fn `UserConstructionScript`)