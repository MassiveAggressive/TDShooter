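; Enemy AI controller that runs BT_Enemy and turns perception updates into blackboard values for tracking the player character.
; Sight of a TDSCharacter sets the target; losing sight clears it and stores the actor's location.
; Hearing and damage stimuli both route through HandleHearing, which sets tracking toward a random navigable point near the stimulus.
; HandleDamage duplicates that logic but is never called.
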(event `self.ReceiveBeginPlay`
  (`self.RunBehaviorTree` "/Game/Blueprints/Enemy/BT_Enemy.BT_Enemy"))

(event `self.AIPerception.OnTargetPerceptionUpdated`
  (params (Actor :type "Actor Object Reference") (Stimulus :type "AIStimulus Structure"))
  (`self.HandleSenses` Actor Stimulus))

(fn `HandleDamage`
  (params (Actor :type "Actor Object Reference") (Stimulus :type "AIStimulus Structure"))
  (bind _randomlocation (`NavigationSystemV1.K2_GetRandomLocationInNavigableRadius` (`.StimulusLocation` (break `AIStimulus` Stimulus)) 500.0 null null))
  (`BlackboardComponent.SetValueAsVector` (`self.Blackboard`) "TargetCharacterLocation" _randomlocation)
  (`BlackboardComponent.SetValueAsBool` (`self.Blackboard`) "IsTracking" true))

(fn `HandleHearing`
  (params (Actor :type "Actor Object Reference") (Stimulus :type "AIStimulus Structure"))
  (bind _randomlocation (`NavigationSystemV1.K2_GetRandomLocationInNavigableRadius` (`.StimulusLocation` (break `AIStimulus` Stimulus)) 500.0 null null))
  (`BlackboardComponent.SetValueAsVector` (`self.Blackboard`) "TargetCharacterLocation" _randomlocation)
  (`BlackboardComponent.SetValueAsBool` (`self.Blackboard`) "IsTracking" true))

(fn `HandleSenses`
  (params (Actor :type "Actor Object Reference") (Stimulus :type "AIStimulus Structure"))
  (bind _returnvalue (`AIPerceptionSystem.GetSenseClassForStimulus` Stimulus))
  (`|ExecutionSequence`
    (:`then_0`
      (if (== _returnvalue "/Script/AIModule.AISense_Sight")
        (`self.HandleSight` (`local.Actor`) (`local.Stimulus`))))
    (:`then_1`
      (if (== _returnvalue "/Script/AIModule.AISense_Hearing")
        (`self.HandleHearing` (`local.Actor`) (`local.Stimulus`))))
    (:`then_2`
      (if (== _returnvalue "/Script/AIModule.AISense_Damage")
        (`self.HandleHearing` (`local.Actor`) (`local.Stimulus`))))))

(fn `HandleSight`
  (params (Actor :type "Actor Object Reference") (Stimulus :type "AIStimulus Structure"))
  (bind _blackboard (`self.Blackboard`))
  (cast `TDSCharacter` Actor)
  (`BlackboardComponent.SetValueAsBool` (`self.Blackboard`) "IsTracking" true)
  (if (`.bSuccessfullySensed` (break `AIStimulus` Stimulus))
    (`BlackboardComponent.SetValueAsObject` (`self.Blackboard`) "TargetCharacter" (`local.Actor`))
    (else
      (`BlackboardComponent.SetValueAsObject` _blackboard "TargetCharacter" null)
      (`BlackboardComponent.SetValueAsVector` _blackboard "TargetCharacterLocation" (`self.K2_GetActorLocation` (`local.Actor`))))))

(fn `UserConstructionScript`)